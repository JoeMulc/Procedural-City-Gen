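; Procedural building actor that generates through a PCG component at BeginPlay, with its height set by proximity to a density point.
; BuildingHeight blends from maximum to minimum as distance from DensityLocation approaches FalloffDistance, plus random variance.
; When PCG generation starts, a flat roof quad is built as a procedural mesh from the first four spline points, raised to that height.
; An unused copy of the roof code sits disconnected in the construction script.
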(event OnPCGGraphStartGeneratingExternal(PCG)
  (params (PCGComponent :type PCG%20Component%20Object%20Reference))
  (Class|ProceduralMeshComponent|CreateMeshSectionLinearColor (Variables|Default|GetRoof) 0 (Utilities|Array|MakeArray (+ (Spline|GetLocationatSplinePoint (Variables|Default|GetSpline) 0 "Local") (Math|Vector|MakeVector 0.0 0.0 (Variables|Default|GetBuildingHeight))) (+ (Spline|GetLocationatSplinePoint (Variables|Default|GetSpline) 1 "Local") (Math|Vector|MakeVector 0.0 0.0 (Variables|Default|GetBuildingHeight))) (+ (Spline|GetLocationatSplinePoint (Variables|Default|GetSpline) 2 "Local") (Math|Vector|MakeVector 0.0 0.0 (Variables|Default|GetBuildingHeight))) (+ (Spline|GetLocationatSplinePoint (Variables|Default|GetSpline) 3 "Local") (Math|Vector|MakeVector 0.0 0.0 (Variables|Default|GetBuildingHeight)))) (Utilities|Array|MakeArray 0 1 2 0 2 3) 0 (Utilities|Array|MakeArray "" "(X=0.000000,Y=1.000000)" "(X=1.000000,Y=0.000000)" "(X=1.000000,Y=1.000000)") 0 0 0 0 0 false false)
  (Rendering|Material|SetMaterial (Variables|Default|GetRoof) 0 "/Game/Assets/Shiny.Shiny"))

(event EventBeginPlay
  (bind _heightvariance (Variables|Default|GetHeightVariance))
  (Variables|Default|SetBuildingHeight (+ (Math|Random|RandomFloatinRange _heightvariance (* _heightvariance -1.0)) (Math|Float|Lerp (Variables|Default|GetMinHeight) (Variables|Default|GetMaxHeight) (- 1.0 (Math|Float|Clamp(Float) (/ (Math|Vector|VectorLength (- (Transformation|GetActorLocation) (Variables|Default|GetDensityLocation))) (Variables|Default|GetFalloffDistance)))))))
  (PCG|Generate (Variables|Default|GetPCG) false))

(event Collision|EventActorBeginOverlap
  (params (OtherActor :type Actor%20Object%20Reference)))

(event EventTick
  (params (DeltaSeconds :type Float%20%28single-precision%29)))

(fn ConstructionScript)