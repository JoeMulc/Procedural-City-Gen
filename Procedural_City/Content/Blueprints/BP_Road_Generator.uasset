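; Procedural road generator that builds a road network and passes it, with its intersections, to a plot generator.
; SummonRoads runs GenerateRoads, calls BuildPlots, then unpauses a looping timer that adds one instanced mesh per segment, animating the network's appearance.
; All three road types share one instanced mesh path; per-actor spawning, spline and building-generation nodes are disconnected.
; ClearRoads destroys tracked road actors and empties the arrays, but leaves mesh instances.
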(event `SummonRoads`
  (set `self.CanGenerateRoads` false)
  (bind (_finnet _intnet) (`self.GenerateRoads`))
  (bind _output_get (set `self.Road Array` _finnet))
  (`/Game/Blueprints/BP_Plot_Generator.BuildPlots` (`self.PlotGenRef`) _output_get _intnet)
  (`KismetSystemLibrary.K2_UnPauseTimerHandle` (`self.TimeHandler`)))

(event `self.ReceiveBeginPlay`
  (bind _returnvalue (`KismetSystemLibrary.K2_SetTimerDelegate` (delegate `DisplayRoads`) 0.005 true))
  (`KismetSystemLibrary.K2_PauseTimerHandle` _returnvalue)
  (set `self.TimeHandler` _returnvalue))

(event `DisplayRoads`
  (bind _index (`self.Index`))
  (bind (_output_start _output_end _output_turnpoint _output_roadtype) (break `Road` (`|GetArrayItem` (`self.Road Array`) _index)))
  (`/Engine/EditorBlueprintResources/StandardMacros.IncrementInt` _index
    (:`  `
      (switch `ERoadType` _output_roadtype
        (:`Main`
          _)
        (:`Secondary`
          _)
        (:`Coastal`
          _))
      (`InstancedStaticMeshComponent.AddInstance` (`self.InstancedStaticMesh`) (`KismetMathLibrary.MakeTransform` _output_start (`KismetMathLibrary.Conv_VectorToRotator` _output_turnpoint)) false)
      (if (> (`self.Index`) (`KismetArrayLibrary.Array_LastIndex` (`self.Road Array`)))
        (`KismetSystemLibrary.K2_PauseTimerHandle` (`self.TimeHandler`))
        (`KismetSystemLibrary.PrintString` "Done" true false (struct :`R` 1.0 :`G` 0.009895 :`A` 1.0) 60.0)
        (set `self.Index` 0)
        (set `self.CanClearRoads` true)))))

(event `ClearRoads`
  (bind _roadactorarray (`self.RoadActorArray`))
  (set `self.CanClearRoads` false)
  (for _array_element _roadactorarray
    (`self.K2_DestroyActor` _array_element))
  (`KismetArrayLibrary.Array_Clear` _roadactorarray)
  (`KismetArrayLibrary.Array_Clear` (`self.Road Array`))
  (set `self.CanGenerateRoads` true))

(fn `UserConstructionScript`)