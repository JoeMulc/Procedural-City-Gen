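; BP_CityPlayer is a player pawn for a road generator scene that shows the UI_RoadGeneratorUI widget on BeginPlay.
; The camera-lock input sets CameraLock and inversely toggles the mouse cursor through BP_CityController.
; SetTopCam and SetFreeCam blend the controller's view target between TopCam and this pawn.
; Movement and camera yaw/pitch input events are empty, as their camera-relative movement and lock-gated rotation logic is disconnected and never runs.
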(event `self.ReceiveBeginPlay`
  (bind _returnvalue (`|CreateWidget` "/Game/CharacteStuff/UI/UI_RoadGeneratorUI.UI_RoadGeneratorUI_C"))
  (bind _output_get (set `self.Veiewport` _returnvalue))
  (`UserWidget.AddToViewport` _output_get 0)
  (set `self.ControllerRef` (`self.GetController`)))

(event `self.ReceiveTick`
  (params (DeltaSeconds :type "Float (single-precision)")))

(event `EnhancedInput|/Game/CharacteStuff/CityInput/IA_Up`
  (params (ActionValue :type "Float (double-precision)") (ElapsedSeconds :type "Float (double-precision)") (TriggeredSeconds :type "Float (double-precision)") (InputAction :type "InputAction Object Reference" :default "/Game/CharacteStuff/CityInput/IA_Up.IA_Up")))

(event `EnhancedInput|/Game/CharacteStuff/CityInput/IA_Sideways`
  (params (ActionValue :type "Float (double-precision)") (ElapsedSeconds :type "Float (double-precision)") (TriggeredSeconds :type "Float (double-precision)") (InputAction :type "InputAction Object Reference" :default "/Game/CharacteStuff/CityInput/IA_Sideways.IA_Sideways")))

(event `EnhancedInput|/Game/CharacteStuff/CityInput/IA_Forward`
  (params (ActionValue :type "Float (double-precision)") (ElapsedSeconds :type "Float (double-precision)") (TriggeredSeconds :type "Float (double-precision)") (InputAction :type "InputAction Object Reference" :default "/Game/CharacteStuff/CityInput/IA_Forward.IA_Forward")))

(event `EnhancedInput|/Game/CharacteStuff/CityInput/IA_CameraYaw`
  (params (ActionValue :type "Float (double-precision)") (ElapsedSeconds :type "Float (double-precision)") (TriggeredSeconds :type "Float (double-precision)") (InputAction :type "InputAction Object Reference" :default "/Game/CharacteStuff/CityInput/IA_CameraYaw.IA_CameraYaw")))

(event `EnhancedInput|/Game/CharacteStuff/CityInput/IA_CameraPitch`
  (params (ActionValue :type "Float (double-precision)") (ElapsedSeconds :type "Float (double-precision)") (TriggeredSeconds :type "Float (double-precision)") (InputAction :type "InputAction Object Reference" :default "/Game/CharacteStuff/CityInput/IA_CameraPitch.IA_CameraPitch")))

(event `EnhancedInput|/Game/CharacteStuff/CityInput/IA_CameraLock`
  (params (ActionValue :type Boolean) (ElapsedSeconds :type "Float (double-precision)") (TriggeredSeconds :type "Float (double-precision)") (InputAction :type "InputAction Object Reference" :default "/Game/CharacteStuff/CityInput/IA_CameraLock.IA_CameraLock"))
  (:`Started`
    (bind _output_get (set `self.CameraLock` ActionValue :!label _label))
    (bind _asbp_city_controller (cast `/Game/CharacteStuff/BP_CityController` (`self.ControllerRef`)))
    (set `PlayerController.bShowMouseCursor` (not _output_get) _asbp_city_controller))
  (:`Completed`
    (goto _label)))

(event `SetTopCam`
  (bind _asbp_city_controller (cast `/Game/CharacteStuff/BP_CityController` (`self.ControllerRef`)))
  (`PlayerController.SetViewTargetWithBlend` _asbp_city_controller (`self.TopCam`) 0.25 "VTBlend_Linear" 0.0 false))

(event `SetFreeCam`
  (bind _asbp_city_controller (cast `/Game/CharacteStuff/BP_CityController` (`self.ControllerRef`)))
  (`PlayerController.SetViewTargetWithBlend` _asbp_city_controller self 0.25 "VTBlend_Linear" 0.0 false))

(fn `UserConstructionScript`)