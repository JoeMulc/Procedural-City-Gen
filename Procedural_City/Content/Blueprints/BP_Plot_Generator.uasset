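; BP_Plot_Generator turns road data into building lots and spawns procedural buildings on them.
; BuildPlots passes the road array to GeneratePlots, splits each plot with SubdivideToLots, and collects the results in LotArray.
; GenerateBuildings spawns a BP_BuildingGrammar per lot at its first point and sets that actor's spline to the lot's points in world space.
; Unconnected leftover chains mostly visualise points with BP_Pillar actors.
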(event `BuildPlots`
  (params (RoadArray :type "Array of Road Structure") (`Intersection Array` :type "Array of Road Structure"))
  (bind _returnvalue (`self.GeneratePlots` RoadArray))
  (for _array_element _returnvalue
    (bind _returnvalue_2 (`self.SubdivideToLots` _array_element))
    (for _array_element_2 _returnvalue_2
      (`KismetArrayLibrary.Array_Add` (`self.LotArray`) _array_element_2))))

(event `Generate Buildings`
  (for _array_element (`self.LotArray`)
    (bind _returnvalue (`|SpawnActorFromClass` "/Game/Grammar/BP_BuildingGrammar.BP_BuildingGrammar_C" (`KismetMathLibrary.Conv_VectorToTransform` (`|GetArrayItem` (break `Lot` _array_element))) "Undefined" "MultiplyWithRoot" null null))
    (`SplineComponent.SetSplinePoints` (`/Game/Grammar/BP_BuildingGrammar.Spline` _returnvalue) (break `Lot` _array_element) "World" true)))

(fn `UserConstructionScript`)